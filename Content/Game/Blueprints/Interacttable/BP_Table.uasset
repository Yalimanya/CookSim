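; BP_Table is an interactable table that holds one object, which a player can place or pick up.
; Grab/Drop places the held object on an empty table, or gives the placed object to an empty-handed player.
; If both are occupied, the placed object handles its own Grab when CanBeGrabbed allows it, freeing the slot.
; Placing attaches the object to ObjectPlace, moves it with MoveComponentTo and clears the player's GrabbedObject.
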(event Custom|Grab
  (params (Player :type BP%20Character%20Object%20Reference))
  (Utilities|IsValid (Variables|Default|GetPlacedObject)
    (:Is%20Valid
      (Default|Grab Player (Variables|Default|GetPlacedObject))
      (Variables|Default|SetPlacedObject 0))))

(event Custom|Place
  (params (Player :type BP%20Character%20Object%20Reference) (ObjectThePlace :type BP%20Grabbable%20Object%20Reference))
  (bind _output_get (Variables|Default|SetPlacedObject ObjectThePlace))
  (Transformation|AttachComponentToComponent _output_get (Variables|Default|GetObjectPlace) "None" "KeepWorld" "KeepWorld" "KeepWorld" true)
  (Components|MoveComponentTo (Variables|/Script/Engine.Actor|GetRootComponent (Variables|Default|GetPlacedObject)) "0, 0, 0" "0, 0, 0" false false 0.2 false)
  (Variables|/Game/Game/Blueprints/BP_Character.BP_Character_C|SetGrabbedObject Player 0))

(event EventBeginPlay)

(event Collision|EventActorBeginOverlap
  (params (OtherActor :type Actor%20Object%20Reference)))

(event EventTick
  (params (DeltaSeconds :type Float%20%28single-precision%29)))

(event EventGrab/Drop
  (params (Player :type BP%20Character%20Object%20Reference))
  (bind (_returnvalue _grabbedobject) (Default|GetGrabbedObject Player))
  (if _returnvalue
    (bind _placedobject (Variables|Default|GetPlacedObject)
      (:then
        (if (Default|CanbeGrabbed _placedobject Player)
          (Default|Grab (Variables|Default|GetPlacedObject) Player)
          (Variables|Default|SetPlacedObject 0)))
      (:else
        (CallFunction|Place Player _grabbedobject)))
    (else
      (CallFunction|Grab Player))))

(fn ConstructionScript)