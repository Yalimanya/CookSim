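; Interactable table where a player slices a placed food item.
; Interact checks that the item can be sliced, changes its state and marks both player and table as interacting.
; Tick advances progress at slicing speed with a debug print, then sets the final state and releases the player at completion.
; Grab/drop works only at zero or full progress and resets it, so partly sliced items stay on the table.
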(event EventBeginPlay
  (|CallParentFunction) ; This node is disabled and will not be called.\nDrag off pins to build functionality.
)

(event Collision|EventActorBeginOverlap
  (params (OtherActor :type Actor%20Object%20Reference))
  (|CallParentFunction OtherActor) ; This node is disabled and will not be called.\nDrag off pins to build functionality.
)

(event EventTick
  (params (DeltaSeconds :type Float%20%28single-precision%29))
  (|CallParentFunction DeltaSeconds)
  (if (Variables|Default|GetIsInteracting)
    (bind _output_get (Variables|Default|SetProgress (Math|Interpolation|FInterptoConstant (Variables|Default|GetProgress) 1.0 DeltaSeconds (Variables|Settings|GetSlicingSpeed))))
    (Development|PrintString (Utilities|String|ToString(Float) _output_get) true true "(R=0.000000,G=0.660000,B=1.000000,A=1.000000)" DeltaSeconds)
    (if (== (Variables|Default|GetProgress) 1.0)
      (CallFunction|StopInteraction)
      (bind _asbp_food_item (Utilities|Casting|CastToBP_FoodItem (Variables|Default|GetPlacedObject)))
      (Default|SetState _asbp_food_item "NewEnumerator2"))))

(event EventGrab/Drop
  (params (Player :type BP%20Character%20Object%20Reference))
  (if (CallFunction|CanGrabObject)
    (|CallParentFunction Player)
    (Variables|Default|SetProgress 0.0)))

(event EventInteract
  (params (Player :type BP%20Character%20Object%20Reference))
  (bind _asbp_food_item (Utilities|Casting|CastToBP_FoodItem (Variables|Default|GetPlacedObject)))
  (if (Default|CanbeSliced _asbp_food_item)
    (Default|SetState _asbp_food_item "NewEnumerator1")
    (Default|SetIsInteracting Player true self)
    (Variables|Default|SetInteractingPlayer Player)
    (Variables|Default|SetIsInteracting true)))

(event EventStopInteraction
  (Variables|Default|SetIsInteracting false)
  (Default|SetIsInteracting (Variables|Default|GetInteractingPlayer) false))

(fn ConstructionScript
  (|CallParentFunction))

(fn CanGrabObject
  (return (or (== (Variables|Default|GetProgress) 0.0) (== (Variables|Default|GetProgress) 1.0))))