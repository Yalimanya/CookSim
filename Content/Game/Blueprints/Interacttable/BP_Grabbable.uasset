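; BP_Grabbable is an interactable physics actor that a player can pick up and drop.
; Grab/Drop acts only if the player holds nothing, turning off the root's physics and collision before passing itself to the player's Grab.
; Drop detaches the actor while keeping its world transform, then restores physics simulation and query-and-physics collision.
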(event Custom|Drop
  (bind _root (Variables|Default|GetRoot))
  (Transformation|DetachFromActor "KeepWorld" "KeepWorld" "KeepWorld")
  (Physics|SetSimulatePhysics _root true)
  (Collision|SetCollisionEnabled _root "QueryAndPhysics"))

(event EventBeginPlay)

(event Collision|EventActorBeginOverlap
  (params (OtherActor :type Actor%20Object%20Reference)))

(event EventTick
  (params (DeltaSeconds :type Float%20%28single-precision%29)))

(event EventGrab/Drop
  (params (Player :type BP%20Character%20Object%20Reference))
  (bind _root (Variables|Default|GetRoot))
  (if (not (.ReturnValue (Default|GetGrabbedObject Player)))
    (Physics|SetSimulatePhysics _root false)
    (Collision|SetCollisionEnabled _root "NoCollision")
    (Default|Grab Player self)))

(fn ConstructionScript)